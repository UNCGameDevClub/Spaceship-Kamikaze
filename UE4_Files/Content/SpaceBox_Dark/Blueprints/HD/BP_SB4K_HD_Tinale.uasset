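; BP_SB4K_HD_Tinale is an HD space skybox actor from the SpaceBox_Dark content, showing the Tinale variant.
; Its construction script scales the whole actor by the Scale variable.
; It then assigns a separate Tinale material to each of six face components: Up, Down, Left, Right, Front and Back.
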(fn `UserConstructionScript`
  (`self.SetActorScale3D` (`self.Scale`))
  (`PrimitiveComponent.SetMaterial` (`self.Up`) 0 "/Game/SpaceBox_Dark/Materials/HD/Tinale/Mat_HD_Tinale_Up.Mat_HD_Tinale_Up")
  (`PrimitiveComponent.SetMaterial` (`self.Right`) 0 "/Game/SpaceBox_Dark/Materials/HD/Tinale/Mat_HD_Tinale_Right.Mat_HD_Tinale_Right")
  (`PrimitiveComponent.SetMaterial` (`self.Left`) 0 "/Game/SpaceBox_Dark/Materials/HD/Tinale/Mat_HD_Tinale_Left.Mat_HD_Tinale_Left")
  (`PrimitiveComponent.SetMaterial` (`self.Front`) 0 "/Game/SpaceBox_Dark/Materials/HD/Tinale/Mat_HD_Tinale_Front.Mat_HD_Tinale_Front")
  (`PrimitiveComponent.SetMaterial` (`self.Down`) 0 "/Game/SpaceBox_Dark/Materials/HD/Tinale/Mat_HD_Tinale_Down.Mat_HD_Tinale_Down")
  (`PrimitiveComponent.SetMaterial` (`self.Back`) 0 "/Game/SpaceBox_Dark/Materials/HD/Tinale/Mat_HD_Tinale_Back.Mat_HD_Tinale_Back"))