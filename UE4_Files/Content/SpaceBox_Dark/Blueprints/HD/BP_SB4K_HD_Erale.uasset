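; BP_SB4K_HD_Erale is a SpaceBox skybox actor that displays the HD Erale environment on six faces.
; Its construction script scales the actor by the Scale variable.
; It then assigns a dedicated Erale material to the first material slot of each Up, Down, Left, Right, Front and Back component.
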(fn `UserConstructionScript`
  (`self.SetActorScale3D` (`self.Scale`))
  (`PrimitiveComponent.SetMaterial` (`self.Up`) 0 "/Game/SpaceBox_Dark/Materials/HD/Erale/Mat_HD_Erale_Up.Mat_HD_Erale_Up")
  (`PrimitiveComponent.SetMaterial` (`self.Right`) 0 "/Game/SpaceBox_Dark/Materials/HD/Erale/Mat_HD_Erale_Right.Mat_HD_Erale_Right")
  (`PrimitiveComponent.SetMaterial` (`self.Left`) 0 "/Game/SpaceBox_Dark/Materials/HD/Erale/Mat_HD_Erale_Left.Mat_HD_Erale_Left")
  (`PrimitiveComponent.SetMaterial` (`self.Front`) 0 "/Game/SpaceBox_Dark/Materials/HD/Erale/Mat_HD_Erale_Front.Mat_HD_Erale_Front")
  (`PrimitiveComponent.SetMaterial` (`self.Down`) 0 "/Game/SpaceBox_Dark/Materials/HD/Erale/Mat_HD_Erale_Down.Mat_HD_Erale_Down")
  (`PrimitiveComponent.SetMaterial` (`self.Back`) 0 "/Game/SpaceBox_Dark/Materials/HD/Erale/Mat_HD_Erale_Back.Mat_HD_Erale_Back"))