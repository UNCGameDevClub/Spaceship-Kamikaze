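; Skybox actor Blueprint for the HD Loriph space background from the SpaceBox_Dark set.
; Its construction script scales the actor by the Scale variable and assigns a dedicated Loriph material to each of six face components: Up, Down, Left, Right, Front and Back.
; The file contains no other logic.
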(fn `UserConstructionScript`
  (`self.SetActorScale3D` (`self.Scale`))
  (`PrimitiveComponent.SetMaterial` (`self.Up`) 0 "/Game/SpaceBox_Dark/Materials/HD/Loriph/Mat_HD_Loriph_Up.Mat_HD_Loriph_Up")
  (`PrimitiveComponent.SetMaterial` (`self.Right`) 0 "/Game/SpaceBox_Dark/Materials/HD/Loriph/Mat_HD_Loriph_Right.Mat_HD_Loriph_Right")
  (`PrimitiveComponent.SetMaterial` (`self.Left`) 0 "/Game/SpaceBox_Dark/Materials/HD/Loriph/Mat_HD_Loriph_Left.Mat_HD_Loriph_Left")
  (`PrimitiveComponent.SetMaterial` (`self.Front`) 0 "/Game/SpaceBox_Dark/Materials/HD/Loriph/Mat_HD_Loriph_Front.Mat_HD_Loriph_Front")
  (`PrimitiveComponent.SetMaterial` (`self.Down`) 0 "/Game/SpaceBox_Dark/Materials/HD/Loriph/Mat_HD_Loriph_Down.Mat_HD_Loriph_Down")
  (`PrimitiveComponent.SetMaterial` (`self.Back`) 0 "/Game/SpaceBox_Dark/Materials/HD/Loriph/Mat_HD_Loriph_Back.Mat_HD_Loriph_Back"))