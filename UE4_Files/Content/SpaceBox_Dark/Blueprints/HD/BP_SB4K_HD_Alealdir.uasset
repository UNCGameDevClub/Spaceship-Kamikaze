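; BP_SB4K_HD_Alealdir is a space skybox actor for the Alealdir HD variant of the SpaceBox Dark set.
; Its construction script sets the actor scale from a Scale variable and assigns a dedicated material to each of the six face components, Up, Down, Left, Right, Front and Back, forming a box backdrop.
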(fn `UserConstructionScript`
  (`self.SetActorScale3D` (`self.Scale`))
  (`PrimitiveComponent.SetMaterial` (`self.Up`) 0 "/Game/SpaceBox_Dark/Materials/HD/Alealdir/Mat_HD_Alealdir_Up.Mat_HD_Alealdir_Up")
  (`PrimitiveComponent.SetMaterial` (`self.Right`) 0 "/Game/SpaceBox_Dark/Materials/HD/Alealdir/Mat_HD_Alealdir_Right.Mat_HD_Alealdir_Right")
  (`PrimitiveComponent.SetMaterial` (`self.Left`) 0 "/Game/SpaceBox_Dark/Materials/HD/Alealdir/Mat_HD_Alealdir_Left.Mat_HD_Alealdir_Left")
  (`PrimitiveComponent.SetMaterial` (`self.Front`) 0 "/Game/SpaceBox_Dark/Materials/HD/Alealdir/Mat_HD_Alealdir_Front.Mat_HD_Alealdir_Front")
  (`PrimitiveComponent.SetMaterial` (`self.Down`) 0 "/Game/SpaceBox_Dark/Materials/HD/Alealdir/Mat_HD_Alealdir_Down.Mat_HD_Alealdir_Down")
  (`PrimitiveComponent.SetMaterial` (`self.Back`) 0 "/Game/SpaceBox_Dark/Materials/HD/Alealdir/Mat_HD_Alealdir_Back.Mat_HD_Alealdir_Back"))