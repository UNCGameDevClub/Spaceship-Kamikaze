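; BP_SB4K_HD_Elmadar is a space skybox actor that displays the HD Elmadar variant from the SpaceBox_Dark content.
; Its construction script sets the actor's 3D scale from the Scale variable.
; It then assigns a matching Elmadar material to the first slot of each of six face components: Up, Down, Left, Right, Front and Back.
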(fn `UserConstructionScript`
  (`self.SetActorScale3D` (`self.Scale`))
  (`PrimitiveComponent.SetMaterial` (`self.Up`) 0 "/Game/SpaceBox_Dark/Materials/HD/Elmadar/Mat_HD_Elmadar_Up.Mat_HD_Elmadar_Up")
  (`PrimitiveComponent.SetMaterial` (`self.Right`) 0 "/Game/SpaceBox_Dark/Materials/HD/Elmadar/Mat_HD_Elmadar_Right.Mat_HD_Elmadar_Right")
  (`PrimitiveComponent.SetMaterial` (`self.Left`) 0 "/Game/SpaceBox_Dark/Materials/HD/Elmadar/Mat_HD_Elmadar_Left.Mat_HD_Elmadar_Left")
  (`PrimitiveComponent.SetMaterial` (`self.Front`) 0 "/Game/SpaceBox_Dark/Materials/HD/Elmadar/Mat_HD_Elmadar_Front.Mat_HD_Elmadar_Front")
  (`PrimitiveComponent.SetMaterial` (`self.Down`) 0 "/Game/SpaceBox_Dark/Materials/HD/Elmadar/Mat_HD_Elmadar_Down.Mat_HD_Elmadar_Down")
  (`PrimitiveComponent.SetMaterial` (`self.Back`) 0 "/Game/SpaceBox_Dark/Materials/HD/Elmadar/Mat_HD_Elmadar_Back.Mat_HD_Elmadar_Back"))