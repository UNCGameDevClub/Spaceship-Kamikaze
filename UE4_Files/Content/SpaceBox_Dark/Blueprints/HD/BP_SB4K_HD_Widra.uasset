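; Space skybox actor from the SpaceBox Dark set that shows the HD Widra sky on six face components.
; The Construction Script sets the actor's scale from the Scale variable.
; It then assigns each face (Up, Down, Left, Right, Front, Back) its matching Widra material in slot 0.
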(fn `UserConstructionScript`
  (`self.SetActorScale3D` (`self.Scale`))
  (`PrimitiveComponent.SetMaterial` (`self.Up`) 0 "/Game/SpaceBox_Dark/Materials/HD/Widra/Mat_HD_Widra_Up.Mat_HD_Widra_Up")
  (`PrimitiveComponent.SetMaterial` (`self.Right`) 0 "/Game/SpaceBox_Dark/Materials/HD/Widra/Mat_HD_Widra_Right.Mat_HD_Widra_Right")
  (`PrimitiveComponent.SetMaterial` (`self.Left`) 0 "/Game/SpaceBox_Dark/Materials/HD/Widra/Mat_HD_Widra_Left.Mat_HD_Widra_Left")
  (`PrimitiveComponent.SetMaterial` (`self.Front`) 0 "/Game/SpaceBox_Dark/Materials/HD/Widra/Mat_HD_Widra_Front.Mat_HD_Widra_Front")
  (`PrimitiveComponent.SetMaterial` (`self.Down`) 0 "/Game/SpaceBox_Dark/Materials/HD/Widra/Mat_HD_Widra_Down.Mat_HD_Widra_Down")
  (`PrimitiveComponent.SetMaterial` (`self.Back`) 0 "/Game/SpaceBox_Dark/Materials/HD/Widra/Mat_HD_Widra_Back.Mat_HD_Widra_Back"))