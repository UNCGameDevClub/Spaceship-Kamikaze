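; BP_SB4K_HD_Saygar is a space skybox actor from the SpaceBox_Dark set, showing the HD Saygar backdrop on six face components.
; Its construction script scales the whole actor by the Scale variable, then assigns a dedicated Saygar material to each of the Up, Down, Left, Right, Front and Back faces.
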(fn `UserConstructionScript`
  (`self.SetActorScale3D` (`self.Scale`))
  (`PrimitiveComponent.SetMaterial` (`self.Up`) 0 "/Game/SpaceBox_Dark/Materials/HD/Saygar/Mat_HD_Saygar_Up.Mat_HD_Saygar_Up")
  (`PrimitiveComponent.SetMaterial` (`self.Right`) 0 "/Game/SpaceBox_Dark/Materials/HD/Saygar/Mat_HD_Saygar_Right.Mat_HD_Saygar_Right")
  (`PrimitiveComponent.SetMaterial` (`self.Left`) 0 "/Game/SpaceBox_Dark/Materials/HD/Saygar/Mat_HD_Saygar_Left.Mat_HD_Saygar_Left")
  (`PrimitiveComponent.SetMaterial` (`self.Front`) 0 "/Game/SpaceBox_Dark/Materials/HD/Saygar/Mat_HD_Saygar_Front.Mat_HD_Saygar_Front")
  (`PrimitiveComponent.SetMaterial` (`self.Down`) 0 "/Game/SpaceBox_Dark/Materials/HD/Saygar/Mat_HD_Saygar_Down.Mat_HD_Saygar_Down")
  (`PrimitiveComponent.SetMaterial` (`self.Back`) 0 "/Game/SpaceBox_Dark/Materials/HD/Saygar/Mat_HD_Saygar_Back.Mat_HD_Saygar_Back"))