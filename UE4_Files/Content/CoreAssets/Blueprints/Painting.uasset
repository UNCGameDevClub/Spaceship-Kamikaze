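; Painting is a configurable wall-art prop that assembles a framed picture in its Construction Script, with no active gameplay logic.
; Size selects the art or canvas mesh, combines with Frame to pick the matching frame mesh, and FrameStyle sets the frame's material.
; A dynamic material instance created from BaseArtMat applies the chosen texture and brightness to the picture, so one Blueprint covers many artwork variants.
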(fn `UserConstructionScript`
  (bind _returnvalue (== (`self.Size`) 1))
  (`StaticMeshComponent.SetStaticMesh` (`self.StaticMesh`) (select `bool` _returnvalue :`false` "/Game/FramedArtandCanvasPack/Meshes/Canvas_01.Canvas_01" :`true` "/Game/FramedArtandCanvasPack/Meshes/Art_001.Art_001" :!type "StaticMesh Object Reference"))
  (`StaticMeshComponent.SetStaticMesh` (`self.StaticMesh1`) (select `bool` _returnvalue :`false` (select `bool` (== (`self.Frame`) 1) :`false` "/Game/FramedArtandCanvasPack/Meshes/Canvas_Frame_02.Canvas_Frame_02" :`true` "/Game/FramedArtandCanvasPack/Meshes/Canvas_Frame_01.Canvas_Frame_01" :!type "StaticMesh Object Reference") :`true` (select `bool` (== (`self.Frame`) 1) :`false` "/Game/FramedArtandCanvasPack/Meshes/Art_Frame_03.Art_Frame_03" :`true` "/Game/FramedArtandCanvasPack/Meshes/Art_Frame_02.Art_Frame_02" :!type "StaticMesh Object Reference")))
  (`PrimitiveComponent.SetMaterial` (`self.StaticMesh1`) 0 (select `int` (`self.FrameStyle`) :`0` "/Game/FramedArtandCanvasPack/Materials/Frames_Brass_Inst.Frames_Brass_Inst" :`1` "/Game/FramedArtandCanvasPack/Materials/Frames_Brass_Inst.Frames_Brass_Inst" :`2` "/Game/FramedArtandCanvasPack/Materials/Frames_BrushedMetal_Inst.Frames_BrushedMetal_Inst" :`3` "/Game/FramedArtandCanvasPack/Materials/Frames_Leather__Inst.Frames_Leather__Inst" :`4` "/Game/FramedArtandCanvasPack/Materials/Frames_Plastic_Inst.Frames_Plastic_Inst" :`5` "/Game/FramedArtandCanvasPack/Materials/Frames_WoodPainted_Inst.Frames_WoodPainted_Inst" :`6` "/Game/FramedArtandCanvasPack/Materials/Frames_WoodVarnished_Inst.Frames_WoodVarnished_Inst" :!type "MaterialInterface Object Reference"))
  (bind _returnvalue_2 (`PrimitiveComponent.CreateDynamicMaterialInstance` (`self.StaticMesh`) 0 "/Game/FramedArtandCanvasPack/Materials/BaseArtMat.BaseArtMat"))
  (`MaterialInstanceDynamic.SetTextureParameterValue` _returnvalue_2 "Picture" (`self.ArtTexture`))
  (`MaterialInstanceDynamic.SetScalarParameterValue` _returnvalue_2 "Brightness" (`self.ArtBrightness`)))